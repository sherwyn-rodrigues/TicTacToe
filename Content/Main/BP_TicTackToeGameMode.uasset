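; Game mode for a Tic-Tac-Toe game that opens the main menu and tracks whose turn it is.
; On BeginPlay it creates the WB_MainMenu widget and adds it to the viewport.
; SwitchPlayer flips IsPlayer1 and sets ColorAndOpacity to red for player one or green for the other player.
; CheckWinCondition takes the player flag but is an empty stub.
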(event Custom|SwitchPlayer
  (bind _output_get (Variables|Default|SetIs%20Player%201 (not (Variables|Default|GetIs%20Player%201))))
  (if _output_get
    (Variables|Default|SetColorAndOpacity (Math|Color|MakeColor 1.0 0.0 0.0))
    (else
      (Variables|Default|SetColorAndOpacity (Math|Color|MakeColor 0.0 1.0 0.0)))))

(event EventBeginPlay
  (bind _returnvalue (UserInterface|CreateWidget "/Game/Main/UI/WB_MainMenu.WB_MainMenu_C"))
  (UserInterface|Viewport|AddtoViewport _returnvalue 0))

(fn ConstructionScript)

(fn CheckWinCondition
  (params (IsPlayer1 :type Boolean)))